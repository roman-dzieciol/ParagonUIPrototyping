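; BP_RadioButtonController makes a group of registered radio buttons behave as a single-choice set.
; Each added button is stored in an array and its state-change event is bound to the controller.
; When one becomes selected, or is chosen by a bounds-checked index, the controller checks it and unchecks all the others.
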(event Custom|OnStateChanged_Event_0
  (params (RadioButton :type W%20Radio%20Button%20Object%20Reference) (bSelected :type Boolean))
  (if bSelected
    (CallFunction|UnselectOtherButtons RadioButton)))

(event Custom|Select%20Button%20At%20Index
  (params (Index :type Integer))
  (bind _checkboxes (Variables|Default|GetCheckboxes))
  (bind _item (Utilities|Array|Get(acopy) _checkboxes Index))
  (if (and (>= Index 0) (< Index (Utilities|Array|Length (Variables|Default|GetCheckboxes))))
    (Default|SetCheckedState _item "Checked")
    (CallFunction|UnselectOtherButtons _item)))

(event Custom|AddRadioButton
  (params (RadioButton :type W%20Radio%20Button%20Object%20Reference))
  (Utilities|Array|Add (Variables|Default|GetCheckboxes) RadioButton)
  (EventDispatchers|AssignOnStateChanged RadioButton (delegate Custom|OnStateChanged_Event_0)))

(fn UnselectOtherButtons
  (params (SelectedButton :type W%20Radio%20Button%20Object%20Reference))
  (for _array_element (Variables|Default|GetCheckboxes)
    (if (!= _array_element SelectedButton)
      (Default|SetCheckedState _array_element "Unchecked")))
  (return))