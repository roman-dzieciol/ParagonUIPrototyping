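; BP_WidgetFuncLibrary is a library of shared helper functions for UMG widgets.
; It picks a checkbox's current style brush from checked, pressed and hovered state, and applies optional textures to images, collapsing them when the texture is invalid.
; It loads key textures from the suffix after an ability name's last underscore, skipping names ending in "Pass".
; It also returns a constructed sample user profile and prints widget state for debugging.
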(fn GetCheckboxCurrentStyle
  (params (Checkbox :type Check%20Box%20Object%20Reference))
  (LocalVariables|SetLocalCheckbox Checkbox)
  (return (Utilities|Select :Index (Class|CheckBox|GetCheckedState (LocalVariables|GetLocalCheckbox)) :Unchecked (select (Class|CheckBox|IsPressed (LocalVariables|GetLocalCheckbox)) (.UncheckedPressedImage (Utilities|Struct|BreakCheckBoxStyle (Variables|/Script/UMG.CheckBox|GetWidgetStyle (LocalVariables|GetLocalCheckbox)))) (select (Widget|IsHovered (LocalVariables|GetLocalCheckbox)) (.UncheckedHoveredImage (Utilities|Struct|BreakCheckBoxStyle (Variables|/Script/UMG.CheckBox|GetWidgetStyle (LocalVariables|GetLocalCheckbox)))) (.UncheckedImage (Utilities|Struct|BreakCheckBoxStyle (Variables|/Script/UMG.CheckBox|GetWidgetStyle (LocalVariables|GetLocalCheckbox)))))) :Checked (select (Class|CheckBox|IsPressed (LocalVariables|GetLocalCheckbox)) (.CheckedPressedImage (Utilities|Struct|BreakCheckBoxStyle (Variables|/Script/UMG.CheckBox|GetWidgetStyle (LocalVariables|GetLocalCheckbox)))) (select (Widget|IsHovered (LocalVariables|GetLocalCheckbox)) (.CheckedHoveredImage (Utilities|Struct|BreakCheckBoxStyle (Variables|/Script/UMG.CheckBox|GetWidgetStyle (LocalVariables|GetLocalCheckbox)))) (.CheckedImage (Utilities|Struct|BreakCheckBoxStyle (Variables|/Script/UMG.CheckBox|GetWidgetStyle (LocalVariables|GetLocalCheckbox)))))) :Undetermined (select (Class|CheckBox|IsPressed (LocalVariables|GetLocalCheckbox)) (.UndeterminedPressedImage (Utilities|Struct|BreakCheckBoxStyle (Variables|/Script/UMG.CheckBox|GetWidgetStyle (LocalVariables|GetLocalCheckbox)))) (select (Widget|IsHovered (LocalVariables|GetLocalCheckbox)) (.UndeterminedHoveredImage (Utilities|Struct|BreakCheckBoxStyle (Variables|/Script/UMG.CheckBox|GetWidgetStyle (LocalVariables|GetLocalCheckbox)))) (.UndeterminedImage (Utilities|Struct|BreakCheckBoxStyle (Variables|/Script/UMG.CheckBox|GetWidgetStyle (LocalVariables|GetLocalCheckbox)))))))))

(fn ApplyOptionalTexturetoImage
  (params (ImageWidget :type Image%20Object%20Reference) (Texture :type Texture%202D%20Object%20Reference))
  (Appearance|SetBrushfromTexture ImageWidget Texture false)
  (Widget|SetVisibility ImageWidget (select (Utilities|IsValid Texture) "SelfHitTestInvisible" "Collapsed")))

(fn LoadKeyTextureforAbilityName
  (params (AbilityName :type String))
  (if (Utilities|String|EndsWith AbilityName "Pass")
    (return 0)
    (else
      (bind _returnvalue (Class|HeroFunctionLibrary|LoadKeyTextureNamed (.RightS (Utilities|String|Split AbilityName "_" "IgnoreCase" "FromEnd"))))
      (return _returnvalue))))

(fn GetUserProfileModel
  (bind _returnvalue (Class|UserProfileFunctionLibrary|ConstructSampleUserProfile))
  (return _returnvalue))

(fn PrintWidgetDebug
  (params (Widget :type Widget%20Object%20Reference) (DebugText :type Text))
  (Development|PrintText 0 (Utilities|Text|FormatText "Widget:{0} Enabled:{1} Hovered:{2} Visibility:{3} {4} {5}" (Utilities|Text|ToText(String) (Utilities|GetDisplayName Widget)) (Utilities|Text|ToText(Boolean) (Class|Widget|GetIsEnabled Widget)) (Utilities|Text|ToText(Boolean) (Widget|IsHovered Widget)) (Utilities|Text|ToText(String) (Utilities|String|EnumtoString (Widget|GetVisibility Widget))) "" DebugText))
  (return))