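; Blueprint function library for card visuals and data, supplying textures and card records by name, type and affinity.
; GetCardBackgroundImage loads a texture named from the sanitized card name, else falls back on type and affinity, with Active and Passive sharing equipment art and Universal defaults.
; GetAllCardsData collects every row of the D_CardsData table.
; GetIconForAffinity maps each affinity to its icon, returning none for Universal.
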(fn GetCardBackgroundImage
  (params (Affinity :type String) (Type :type String) (CardName :type String))
  (bind _returnvalue (Utilities|String|Append Type "." Affinity))
  (bind _returnvalue_2 (Class|CardsFunctionLibrary|MakeValidTableRowName (Utilities|String|Replace (Utilities|String|Replace (Utilities|String|Replace CardName " of " " Of " "CaseSensitive") " the " " The " "CaseSensitive") "-")))
  (bind _returnvalue_3 (Class|CardsFunctionLibrary|LoadCardTextureNamed (Utilities|String|ToString(Name) _returnvalue_2)))
  (if (Utilities|IsValid _returnvalue_3)
    (return _returnvalue_3)
    (elif (Utilities|Enum|Equal(Enum) _returnvalue "Active.Intellect")
      (return "/Game/Art/Cards/T_EquipmentIntellect.T_EquipmentIntellect")
      (elif (Utilities|Enum|Equal(Enum) _returnvalue "Passive.Intellect")
        (return "/Game/Art/Cards/T_EquipmentIntellect.T_EquipmentIntellect")
        (elif (Utilities|Enum|Equal(Enum) _returnvalue "Upgrade.Intellect")
          (return "/Game/Art/Cards/T_UpgradeIntellect.T_UpgradeIntellect")
          (elif (Utilities|Enum|Equal(Enum) _returnvalue "Active.Corruption")
            (return "/Game/Art/Cards/T_EquipmentCorruption.T_EquipmentCorruption")
            (elif (Utilities|Enum|Equal(Enum) _returnvalue "Passive.Corruption")
              (return "/Game/Art/Cards/T_EquipmentCorruption.T_EquipmentCorruption")
              (elif (Utilities|Enum|Equal(Enum) _returnvalue "Upgrade.Corruption")
                (return "/Game/Art/Cards/T_UpgradeCorruption.T_UpgradeCorruption")
                (elif (Utilities|Enum|Equal(Enum) _returnvalue "Active.Growth")
                  (return "/Game/Art/Cards/T_EquipmentGrowth.T_EquipmentGrowth")
                  (elif (Utilities|Enum|Equal(Enum) _returnvalue "Passive.Growth")
                    (return "/Game/Art/Cards/T_EquipmentGrowth.T_EquipmentGrowth")
                    (elif (Utilities|Enum|Equal(Enum) _returnvalue "Upgrade.Growth")
                      (return "/Game/Art/Cards/T_UpgradeGrowth.T_UpgradeGrowth")
                      (elif (Utilities|Enum|Equal(Enum) _returnvalue "Active.Order")
                        (return "/Game/Art/Cards/T_EquipmentOrder.T_EquipmentOrder")
                        (elif (Utilities|Enum|Equal(Enum) _returnvalue "Passive.Order")
                          (return "/Game/Art/Cards/T_EquipmentOrder.T_EquipmentOrder")
                          (elif (Utilities|Enum|Equal(Enum) _returnvalue "Upgrade.Order")
                            (return "/Game/Art/Cards/T_UpgradeOrder.T_UpgradeOrder")
                            (elif (Utilities|Enum|Equal(Enum) _returnvalue "Active.Fury")
                              (return "/Game/Art/Cards/T_EquipmentFury.T_EquipmentFury")
                              (elif (Utilities|Enum|Equal(Enum) _returnvalue "Passive.Fury")
                                (return "/Game/Art/Cards/T_EquipmentFury.T_EquipmentFury")
                                (elif (Utilities|Enum|Equal(Enum) _returnvalue "Upgrade.Fury")
                                  (return "/Game/Art/Cards/T_UpgradeFury.T_UpgradeFury")
                                  (elif (Utilities|Enum|Equal(Enum) Type "Upgrade")
                                    (return "/Game/Art/Cards/T_UpgradeUniveral.T_UpgradeUniveral")
                                    (else
                                      (return "/Game/Art/Cards/T_EquipmentUniversal.T_EquipmentUniversal"))))))))))))))))))))

(fn GetAllCardsData
  (bind _result (LocalVariables|GetResult))
  (bind _outrownames (DataTable|GetDataTableRowNames "/Game/Data/D_CardsData.D_CardsData"))
  (for _array_element _outrownames
    (bind _returnvalue (Utilities|GetDataTableRow "/Game/Data/D_CardsData.D_CardsData" _array_element)
      (:then
        (Utilities|Array|Add _result _returnvalue))))
  (return _result))

(fn GetIconforAffinity
  (params (Affinity :type String))
  (switch string Affinity
    (:Default
      _)
    (:Order
      (return "/Game/Art/Affinity/T_Order_Affinity_Icon.T_Order_Affinity_Icon"))
    (:Growth
      (return "/Game/Art/Affinity/T_Growth_Affinity_Icon.T_Growth_Affinity_Icon"))
    (:Intellect
      (return "/Game/Art/Affinity/T_Intellect_Affinity_Icon.T_Intellect_Affinity_Icon"))
    (:Corruption
      (return "/Game/Art/Affinity/T_Corruption_Affinity_Icon.T_Corruption_Affinity_Icon"))
    (:Fury
      (return "/Game/Art/Affinity/T_Fury_Affinity_Icon.T_Fury_Affinity_Icon"))
    (:Universal
      _))
  (return 0))